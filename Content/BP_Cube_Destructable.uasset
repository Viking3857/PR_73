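; BP_Cube_Destructable is a cube actor that shrinks each time another actor begins overlapping it.
; At BeginPlay it stores five percent of its starting scale as a fixed reduction step.
; Each overlap subtracts that step, so shrinking is linear, with no lower limit or destroy call in this Blueprint.
; Tick is disabled, and the construction script only calls its parent.
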(event `self.ReceiveBeginPlay`
  (set `self.Reduction` (* (`self.GetActorScale3D`) 0.05))
  (`parent.ReceiveBeginPlay`))

(event `self.ReceiveActorBeginOverlap`
  (params (OtherActor :type "Actor Object Reference"))
  (`self.SetActorScale3D` (- (`self.GetActorScale3D`) (`self.Reduction`)))
  (`parent.ReceiveActorBeginOverlap` null))

(fn `UserConstructionScript`
  (`parent.UserConstructionScript`))